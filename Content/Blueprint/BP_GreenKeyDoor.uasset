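; BP_GreenKeyDoor is an interactable door that acts as a step in the quest sequence, opening only at a specific stage.
; CanInteract adds a check to the parent's rule, requiring the QuestionSubsystem's current quest index to equal a hardcoded value.
; Interact runs the parent behavior, plays the door-opening sound in 2D and advances the subsystem to the next quest.
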(event `self.Interact`
  (params (Interactor :type "Actor Object Reference"))
  (`parent.Interact` Interactor)
  (`GameplayStatics.PlaySound2D` "/Game/SFX/Open-Door.Open-Door" 1.0 1.0 0.0 null null)
  (`QuestionSubsystem.NextQuest` (subsystem `QuestionSubsystem`)))

(fn `CanInteract`
  (params (Interactor :type "Actor Object Reference"))
  (returns (ReturnValue :type Boolean))
  (bind _returnvalue (`parent.CanInteract` Interactor))
  (return (and _returnvalue (== (`QuestionSubsystem.GetCurrentQuestIndex` (subsystem `QuestionSubsystem`)) 7))))

(fn `UserConstructionScript`)