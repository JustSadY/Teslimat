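; BP_Table is an interactable table where the player drops off a carried pizza as a quest step.
; CanInteract allows use only while the QuestionSubsystem's current quest index is 2, calling the parent check but ignoring its result.
; On Interact, it hides the pizza on the TeslimatCharacter, shows its own Pizza component, advances to the next quest and closes the ClosedDoor.
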(event `self.Interact`
  (params (Interactor :type "Actor Object Reference"))
  (bind _asteslimat_character (cast `TeslimatCharacter` Interactor))
  (`/Engine/EditorBlueprintResources/StandardMacros.IsValid` _asteslimat_character
    (:`Is Valid`
      (`TeslimatCharacter.SetVisiblePizza` _asteslimat_character false)
      (`SceneComponent.SetVisibility` (`self.Pizza`) true false)
      (`QuestionSubsystem.NextQuest` (subsystem `QuestionSubsystem`))
      (`DoorActor.CloseDoor` (`self.ClosedDoor`)))))

(fn `CanInteract`
  (params (Interactor :type "Actor Object Reference"))
  (returns (ReturnValue :type Boolean))
  (`parent.CanInteract` Interactor)
  (return (== (`QuestionSubsystem.GetCurrentQuestIndex` (subsystem `QuestionSubsystem`)) 2)))

(fn `UserConstructionScript`)