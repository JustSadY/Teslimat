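; BP_TVOFON is a trigger actor that turns on a TV panel at a specific point in the quest progression.
; When a Character enters its Box, it checks a first-time flag and whether the quest subsystem reports quest index 7.
; If both hold, it clears the flag and calls OpenTV on the referenced TVPanel, so it fires only once.
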(event `self.Box.OnComponentBeginOverlap`
  (params (OverlappedComponent :type "PrimitiveComponent Object Reference") (OtherActor :type "Actor Object Reference") (OtherComp :type "PrimitiveComponent Object Reference") (OtherBodyIndex :type Integer) (bFromSweep :type Boolean) (SweepResult :type "HitResult Structure (by ref)"))
  (cast `Character` OtherActor)
  (if (and (`self.BIsFirst`) (== (`QuestionSubsystem.GetCurrentQuestIndex` (subsystem `QuestionSubsystem`)) 7))
    (set `self.BIsFirst` false)
    (`/Engine/EditorBlueprintResources/StandardMacros.IsValid` (`self.TVPanel`)
      (:`Is Valid`
        (`/Game/Blueprint/TVPanel.OpenTV` (`self.TVPanel`))))))

(fn `UserConstructionScript`)