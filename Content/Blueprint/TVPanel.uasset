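; TVPanel is an interactable TV panel that plays a positional sound while open until an interaction closes it.
; OpenTV, which nothing in this Blueprint calls, hides the static mesh and stores the spawned sound if not already open.
; Interact calls CloseTV, which shows the mesh again and stops that sound.
; CanInteract returns only the open flag, ignoring the parent's result.
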(event `self.Interact`
  (params (Interactor :type "Actor Object Reference"))
  (`self.CloseTV`))

(fn `CanInteract`
  (params (Interactor :type "Actor Object Reference"))
  (returns (ReturnValue :type Boolean))
  (`parent.CanInteract` Interactor)
  (return (`self.BIsopen`)))

(fn `CloseTV`
  (set `self.BIsopen` false)
  (`SceneComponent.SetVisibility` (`self.StaticMesh`) true false)
  (`AudioComponent.Stop` (`self.ActiveSound`)))

(fn `OpenTV`
  (if (not (`self.BIsopen`))
    (set `self.BIsopen` true)
    (`SceneComponent.SetVisibility` (`self.StaticMesh`) false false)
    (bind _returnvalue (`GameplayStatics.SpawnSoundAtLocation` (`self.Sound`) (`SceneComponent.GetSocketLocation` (`self.StaticMesh`) "None") (struct) 0.5 1.0 0.0 "/Game/SFX/SA_Location.SA_Location" null))
    (set `self.ActiveSound` _returnvalue)))

(fn `UserConstructionScript`)